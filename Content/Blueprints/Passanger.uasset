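; Passenger character with food and stamina needs, driven by an AI controller and blackboard, that can occupy work stations.
; Tick uses Delays to periodically apply stat deltas; critical levels add ailments, and zero triggers death, which unpossesses the AI.
; SetPriorityAilment selects among active ailments via math expressions comparing food, stamina and oxygen, then writes it to the blackboard.
; SetStation assigns the WorkPlace key and evicts the station's previous user; HaveSkill searches the skill list.
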(event Custom|Death_Event
  (if (not (Variables|VitalsModifications|GetDie))
    (Variables|VitalsModifications|SetDie true)
    (Pawn|UnPossess (AI|GetAIController self))))

(event EventTick
  (params (DeltaSeconds :type Float%20%28single-precision%29))
  (if (not (Variables|VitalsModifications|GetDie))
    (Development|PrintString (Utilities|String|ToString(Text) (Utilities|Text|FormatText "Stamina: {0} Food: {1}" (Variables|Vitals|GetStamina) (Variables|Vitals|GetFood))))
    (Utilities|FlowControl|Sequence
      (:then_0
        (Variables|Default|SetPriorityAilment "NewEnumerator3"))
      (:then_1
        (Utilities|FlowControl|Delay (Variables|Vitals|GetFoodPause))
        (StatsModified|AddFood (Variables|Vitals|GetFoodDelta)))
      (:then_2
        (Utilities|FlowControl|Delay (Variables|Vitals|GetStaminaPause))
        (StatsModified|AddStamina (Variables|Vitals|GetStaminaDelta))))))

(event EventBeginPlay
  (StatsModified|AddFood 0.0)
  (StatsModified|AddStamina 0.0)
  (EventDispatchers|BindEventtoDeathEvent (delegate Custom|Death_Event)))

(fn ConstructionScript
  (Variables|/Script/Engine.CharacterMovementComponent|SetMaxWalkSpeed (Variables|Character|GetCharacterMovement) 2e+02))

(fn AddStamina
  (params (Delta :type Float%20%28single-precision%29))
  (bind _ailments (Variables|Default|GetAilments))
  (if (not (Variables|VitalsModifications|GetBlockStamina))
    (Variables|Vitals|SetStamina (+ (Variables|Vitals|GetStamina) Delta))
    (if (<= (Variables|Vitals|GetStamina) (Variables|VitalsModifications|GetCritical%20Level))
      (Utilities|Array|AddUnique _ailments "NewEnumerator1")
      (CallFunction|SetPriorityAilment)
      (if (<= (Variables|Vitals|GetStamina) 0.0)
        (Default|CallDeathEvent))
      (else
        (Utilities|Array|RemoveItem _ailments "NewEnumerator1")))))

(fn AddFood
  (params (Delta :type Float%20%28single-precision%29))
  (bind _ailments (Variables|Default|GetAilments))
  (if (not (Variables|VitalsModifications|GetBlockFood))
    (Variables|Vitals|SetFood (+ (Variables|Vitals|GetFood) Delta))
    (if (<= (Variables|Vitals|GetFood) (Variables|VitalsModifications|GetCritical%20Level))
      (Utilities|Array|AddUnique _ailments "NewEnumerator0")
      (CallFunction|SetPriorityAilment)
      (if (<= (Variables|Vitals|GetFood) 0.0)
        (Default|CallDeathEvent))
      (else
        (Utilities|Array|RemoveItem _ailments "NewEnumerator0")))))

(fn SetStation
  (params (Station :type BP%20Work%20Station%20Object%20Reference))
  (bind _returnvalue (Utilities|Name|MakeLiteralName "WorkPlace"))
  (bind _self self)
  (bind _returnvalue_2 (AI|GetAIController _self))
  (bind _blackboard (Variables|/Script/AIModule.AIController|GetBlackboard _returnvalue_2))
  (bind _returnvalue_3 (AI|Components|Blackboard|GetValueasObject _blackboard _returnvalue))
  (bind (_asbp_station _bsuccess) (Utilities|Casting|CastToBP_Station _returnvalue_3))
  (if _bsuccess
    (if (!= Station _asbp_station)
      (Variables|/Game/Blueprints/BP_Station.BP_Station_C|SetUser _asbp_station 0)
      (bind _user (Variables|/Game/Blueprints/BP_Station.BP_Station_C|GetUser Station :!label _label)
        (:then
          (CallFunction|ClearStation _user))
        (:else
          _))
      (Variables|/Game/Blueprints/BP_Station.BP_Station_C|SetUser Station self)
      (AI|Components|Blackboard|SetValueasObject _blackboard (Utilities|Name|MakeLiteralName "WorkPlace") Station))
    (else
      (goto _label))))

(fn ClearStation
  (bind _self self)
  (bind _returnvalue (AI|GetAIController _self))
  (bind _blackboard (Variables|/Script/AIModule.AIController|GetBlackboard _returnvalue))
  (AI|Components|Blackboard|ClearValue _blackboard (Utilities|Name|MakeLiteralName "WorkPlace"))
  (AI|Components|Blackboard|ClearValue _blackboard (Utilities|Name|MakeLiteralName "TargetVector")))

(fn HaveSkill
  (params (Skillg :type ESkillls%20Enum :default "NewEnumerator0"))
  (bind _array_element (Utilities|Array|ForEachLoopwithBreak (Variables|Default|GetSkills) :!label _label)
    (:LoopBody
      (if (Utilities|Enum|Equal(Enum) _array_element Skillg)
        (goto _label Break)))
    (:Completed
      (return (Utilities|Enum|Equal(Enum) _array_element Skillg)))))

(fn SetPriorityAilment
  (if (not (Variables|VitalsModifications|GetDie))
    (Variables|Default|SetPriorityAilment "NewEnumerator3")
    (for _array_element (Variables|Default|GetAilments)
      (switch Utilities|FlowControl|Switch|SwitchonEAilments _array_element
        (:NewEnumerator0
          (if (|(({CA4AA9C2-4525-7258-3D68-91BAC5F1D5D5}<={73A4FCAD-4A04-E364-24AC-5BA98135FA8B})&&({CA4AA9C2-4525-7258-3D68-91BAC5F1D5D5}<={4C3B4F86-4954-93C8-1B4D-0FB8AB65E6E2})))
            (Variables|Default|SetPriorityAilment "NewEnumerator0")))
        (:NewEnumerator1
          (if (|(({73A4FCAD-4A04-E364-24AC-5BA98135FA8B}<={CA4AA9C2-4525-7258-3D68-91BAC5F1D5D5})&&({73A4FCAD-4A04-E364-24AC-5BA98135FA8B}<={4C3B4F86-4954-93C8-1B4D-0FB8AB65E6E2})))
            (Variables|Default|SetPriorityAilment "NewEnumerator1")))
        (:NewEnumerator2
          (if (|(({4C3B4F86-4954-93C8-1B4D-0FB8AB65E6E2}<={CA4AA9C2-4525-7258-3D68-91BAC5F1D5D5})&&({4C3B4F86-4954-93C8-1B4D-0FB8AB65E6E2}<={73A4FCAD-4A04-E364-24AC-5BA98135FA8B})))
            (Variables|Default|SetPriorityAilment "NewEnumerator2")))))
    (bind (_blackboardcomponent _returnvalue) (Class|AIController|UseBlackboard (AI|GetAIController self) "/Game/AI/HellBoard.HellBoard"))
    (if _returnvalue
      (AI|Components|Blackboard|SetValueasEnum _blackboardcomponent (Utilities|Name|MakeLiteralName "PriorityAilment") (Variables|Default|GetPriorityAilment)))))