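; BP_Station is a placeable grid structure that starts unbuilt and becomes finished when its build task completes.
; On placement it gets the TaskList from its widget, applies a placed-state material and adds a BP_Task tagged as build work.
; The task's completion event marks the station built, removes the task, refreshes the list and swaps in the final material.
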(event `self.OnPlaced`
  (`parent.OnPlaced`)
  ;[0 0.005394 1 0.295] InitTaskList
  (bind _astask_list (cast `/Game/Blueprints/Structures/TaskList` (`WidgetComponent.GetWidget` (`self.Widget`))))
  (set `self.TaskList` _astask_list)
  (if (not (`self.IsBuilt`))
    (`PrimitiveComponent.SetMaterial` (`self.StaticMesh`) 0 "/Game/Materials/GridActorMatAfterPlaced.GridActorMatAfterPlaced")
    (bind _returnvalue (`self.Add Task` (delegate `OnBuilt`)))))

(event `OnBuilt`
  (set `self.IsBuilt` true)
  (`KismetArrayLibrary.Array_RemoveItem` (`self.Tasks`) (stale `self.OnPlaced` _returnvalue))
  (`/Game/Blueprints/Structures/TaskList.Update` (`self.TaskList`) (`self.Tasks`))
  (`PrimitiveComponent.SetMaterial` (`self.StaticMesh`) 0 (`self.FinalMaterial`)))

(fn `Add Task`
  (params (OnCompleted :type "Delegate (by ref)"))
  (returns (ReturnValue :type "/Game/Blueprints/Task/BP_Task Object Reference"))
  (bind _returnvalue (`|GenericCreateObject` "/Game/Blueprints/Task/BP_Task.BP_Task_C" self (`|FormatText` "Build {name}" (`self.Name`)) false 5.0 (`|MakeMap` "NewEnumerator0" :!type "/Game/Blueprints/Task/Resources Enum") (struct :`TagName` "Task.Work.Build")))
  (add `/Game/Blueprints/Task/BP_Task.OnCompleted` _returnvalue OnCompleted)
  (`KismetArrayLibrary.Array_AddUnique` (`self.Tasks`) _returnvalue)
  (`/Game/Blueprints/Structures/TaskList.Update` (`self.TaskList`) (`self.Tasks`))
  (return _returnvalue))

(fn `UserConstructionScript`
  (`parent.UserConstructionScript`))