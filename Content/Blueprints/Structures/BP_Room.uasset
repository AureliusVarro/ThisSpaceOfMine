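; BP_Room is a room structure with a finite oxygen level that the crewmates inside it consume.
; A box overlap query on BeginPlay seeds the list of occupants, and actor overlap events keep it current.
; Each tick, living occupants draw oxygen in turn at their own per-second rate, scaled by delta time and capped by what remains.
; The amount given to each crewmate is subtracted from the room, and nothing here replenishes it.
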(event `self.ReceiveBeginPlay`
  (bind _box (`self.Box`))
  (bind _outactors (`KismetSystemLibrary.BoxOverlapActors` (`SceneComponent.K2_GetComponentLocation` _box) (`BoxComponent.BoxExtent` _box) (`|MakeArray` "ObjectTypeQuery3" :!type "EObjectTypeQuery Enum") "/Game/Blueprints/Crewmates/Crewmate.Crewmate_C"))
  (for _array_element _outactors
    (bind _ascrewmate (cast `/Game/Blueprints/Crewmates/Crewmate` _array_element))
    (`KismetArrayLibrary.Array_Add` (`self.CrewmatesInRoom`) _ascrewmate)))

(event `self.ReceiveActorBeginOverlap`
  (params (OtherActor :type "Actor Object Reference"))
  (bind _ascrewmate (cast `/Game/Blueprints/Crewmates/Crewmate` OtherActor))
  (`KismetArrayLibrary.Array_AddUnique` (`self.CrewmatesInRoom`) _ascrewmate))

(event `self.ReceiveActorEndOverlap`
  (params (OtherActor :type "Actor Object Reference"))
  (bind _ascrewmate (cast `/Game/Blueprints/Crewmates/Crewmate` OtherActor))
  (`KismetArrayLibrary.Array_RemoveItem` (`self.CrewmatesInRoom`) _ascrewmate))

(event `self.ReceiveTick`
  (params (DeltaSeconds :type "Float (single-precision)"))
  (for _array_element (`self.CrewmatesInRoom`)
    (`self.CalculateOxygen` _array_element)))

(fn `CalculateOxygen`
  (params (Man :type "/Game/Blueprints/Crewmates/Crewmate Object Reference"))
  (bind _returnvalue (`KismetMathLibrary.FClamp` (* (`/Game/Blueprints/Crewmates/Crewmate.OxygenPerSecond` Man) -1.0 (`GameplayStatics.GetWorldDeltaSeconds`)) 0.0 (`self.OxygenLevel`)))
  (if (not (`/Game/Blueprints/Crewmates/Crewmate.IsDead` Man))
    (`/Game/Blueprints/Crewmates/Crewmate.Add Oxygen` Man _returnvalue)
    (set `self.OxygenLevel` (- (`self.OxygenLevel`) _returnvalue))))

(fn `UserConstructionScript`)