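; RTS camera that also serves as the player's controller for passengers and object placement, and creates the HUD.
; Axis input, screen edges, middle-mouse drag and wheel drive panning, orbiting and spring-arm zoom.
; Clicks select passengers with custom-depth highlighting; right-click toggles blackboard-flagged control, letting held left-click steer them via AI move.
; Number keys spawn buildables that follow the cursor on a looping timer, grid-snapped over floors, rotatable until placed.
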(event `self.ReceiveBeginPlay`
  ;[1 1 1] Begin Play Show Cursor
  (set `PlayerController.bShowMouseCursor` true (`GameplayStatics.GetPlayerController` 0))
  (`self.LockMouseToViewPort`)
  ;[1 1 1] Init UI
  (bind _returnvalue (`|CreateWidget` "/Game/Blueprints/UI/HUD.HUD_C"))
  (bind _output_get (set `self.HUD_Ref` _returnvalue))
  (`UserWidget.AddToViewport` _output_get 0)
  (bind _asbp_game_mode (cast `/Game/Blueprints/BP_Gamemode` (`GameplayStatics.GetGameMode`)))
  (`/Game/Blueprints/BP_Gamemode.InitHUD` _asbp_game_mode (`self.HUD_Ref`)))

(event `InputAxis|MoveForward`
  (params (AxisValue :type "Float (single-precision)"))
  ;[1 1 1] Camera Movements WASD
  (`self.K2_AddActorLocalOffset` (`KismetMathLibrary.MakeVector` (* AxisValue (`self.Camera_MoveSpeed`))) true)
  (if (or (!= AxisValue 0.0) (!= (stale `InputAxis|MoveRight` AxisValue) 0.0)) :!label _label
    _))

(event `InputAxisKey|MouseX`
  (params (AxisValue :type "Float (single-precision)"))
  ;[1 1 1] Mouse X and Y
  (`self.RotateX` AxisValue)
  (`self.ScreenEdgeHitX`))

(event `InputAxisKey|MouseY`
  (params (AxisValue :type "Float (single-precision)"))
  ;[1 1 1] Mouse X and Y
  (`self.RotateY` AxisValue)
  (`self.ScreenEdgeHitY`))

(event `InputAxis|MoveRight`
  (params (AxisValue :type "Float (single-precision)"))
  ;[1 1 1] Camera Movements WASD
  (`self.K2_AddActorLocalOffset` (`KismetMathLibrary.MakeVector` 0.0 (* AxisValue (`self.Camera_MoveSpeed`))) true)
  (goto _label))

(event `RotateX`
  (params (InValueX :type "Float (double-precision)"))
  ;[1 1 1] Rotate
  (`/Engine/EditorBlueprintResources/StandardMacros.Gate` true :!label _label_2
    (:`Exit`
      (`self.K2_AddActorLocalRotation` (`KismetMathLibrary.MakeRotator` 0.0 0.0 (* InValueX (`self.Camera_RotateSpeed`)))))))

(event `Key|MouseScrollUp`
  (params (Key :type "Key Structure"))
  (bind _springarm (`self.SpringArm`))
  ;[1 1 1] Zoom In And Out
  (:`Pressed`
    ;;[1 1 1] Zoom In By Arm Length
    (set `SpringArmComponent.TargetArmLength` (`KismetMathLibrary.FClamp` (- (`SpringArmComponent.TargetArmLength` _springarm) (`self.Camera_ZoomSpeed`)) 500.0 5000.0) _springarm)))

(event `Key|MiddleMouseButton`
  (params (Key :type "Key Structure"))
  (bind (_returnvalue_roll _returnvalue_pitch _returnvalue_yaw) (`KismetMathLibrary.BreakRotator` (`SceneComponent.K2_GetComponentRotation` (`self.Camera`))))
  ;[1 1 1] Rotate
  (:`Pressed`
    (set `self.Camera_ScreenEdgeHitEnabled` false)
    (`|ExecutionSequence`
      (:`then_0`
        (goto _label_2 :!via `Open`))
      (:`then_1`
        (goto _label_3 :!via `Open`))))
  (:`Released`
    (set `self.Camera_ScreenEdgeHitEnabled` true)
    (`|ExecutionSequence`
      (:`then_0`
        (goto _label_2 :!via `Close`))
      (:`then_1`
        (goto _label_3 :!via `Close`)))))

(event `ScreenEdgeHitX`
  (bind _camera_screenedgehitspeed (`self.Camera_ScreenEdgeHitSpeed`))
  (bind (_x _y) (`KismetMathLibrary.BreakVector2D` (`WidgetLayoutLibrary.GetViewportSize`)))
  (bind _returnvalue (/ (- _x (`PlayerController.GetMousePosition` (`GameplayStatics.GetPlayerController` 0))) _x))
  ;[1 1 1] Screen Edge Hit
  (if (`self.Camera_ScreenEdgeHitEnabled`)
    (`|ExecutionSequence`
      (:`then_0`
        (if (>= _returnvalue 0.98)
          (`self.K2_AddActorLocalOffset` (`KismetMathLibrary.MakeVector` 0.0 (* -1 _camera_screenedgehitspeed)) true)))
      (:`then_1`
        (if (<= _returnvalue 0.02)
          (`self.K2_AddActorLocalOffset` (`KismetMathLibrary.MakeVector` 0.0 _camera_screenedgehitspeed) true))))))

(event `RotateY`
  (params (InValueY :type "Float (double-precision)"))
  (bind (_returnvalue_roll _returnvalue_pitch _returnvalue_yaw) (`KismetMathLibrary.BreakRotator` (`SceneComponent.K2_GetComponentRotation` (`self.Camera`))))
  ;[1 1 1] Rotate
  (`/Engine/EditorBlueprintResources/StandardMacros.Gate` true :!label _label_3
    (:`Exit`
      ;;[1 1 1] Focal Point Rotation
      (`SceneComponent.K2_SetWorldRotation` (`self.SpringArm`) (`KismetMathLibrary.MakeRotator` _returnvalue_roll (`KismetMathLibrary.FClamp` (+ (* InValueY (`self.Camera_RotateSpeed`)) _returnvalue_pitch) -89.0 -10.0) _returnvalue_yaw) false false))))

(event `ScreenEdgeHitY`
  (bind _camera_screenedgehitspeed (`self.Camera_ScreenEdgeHitSpeed`))
  (bind (_x _y) (`KismetMathLibrary.BreakVector2D` (`WidgetLayoutLibrary.GetViewportSize`)))
  (bind _returnvalue (/ (- _y (`.LocationY` (`PlayerController.GetMousePosition` (`GameplayStatics.GetPlayerController` 0)))) _y))
  ;[1 1 1] Screen Edge Hit
  (if (`self.Camera_ScreenEdgeHitEnabled`)
    (`|ExecutionSequence`
      (:`then_0`
        (if (>= _returnvalue 0.98)
          (`self.K2_AddActorLocalOffset` (`KismetMathLibrary.MakeVector` _camera_screenedgehitspeed) true)))
      (:`then_1`
        (if (<= _returnvalue 0.02)
          (`self.K2_AddActorLocalOffset` (`KismetMathLibrary.MakeVector` (* -1 _camera_screenedgehitspeed)) true))))))

(event `Key|MouseScrollDown`
  (params (Key :type "Key Structure"))
  (bind _springarm (`self.SpringArm`))
  ;[1 1 1] Zoom In And Out
  (:`Pressed`
    ;;[1 1 1] Zoom Out By Arm Length
    (set `SpringArmComponent.TargetArmLength` (`KismetMathLibrary.FClamp` (+ (`SpringArmComponent.TargetArmLength` _springarm) (`self.Camera_ZoomSpeed`)) 500.0 5000.0) _springarm)))

(event `self.ReceiveTick`
  (params (DeltaSeconds :type "Float (single-precision)"))
  (if (`self.Controlling`)
    (`/Engine/EditorBlueprintResources/StandardMacros.Gate` true :!label _label_4 ; While key is pressed...
      (:`Exit`
        (`self.MovePassenger` (`PlayerController.GetHitResultUnderCursorByChannel` (`GameplayStatics.GetPlayerController` 0) "TraceTypeQuery1" true))))))

(event `LockMouseToViewPort`
  ;[1 1 1] Lock And Release Mouse
  (`WidgetBlueprintLibrary.SetInputMode_GameAndUIEx` (`GameplayStatics.GetPlayerController` 0) null "LockAlways" false))

(event `Key|LeftMouseButton`
  (params (Key :type "Key Structure"))
  (:`Pressed`
    (goto _label_4 :!via `Open`))
  (:`Released`
    (goto _label_4 :!via `Close`)))

(event `ReleaseMouse`
  ;[1 1 1] Lock And Release Mouse
  (`WidgetBlueprintLibrary.SetInputMode_GameAndUIEx` (`GameplayStatics.GetPlayerController` 0) null "DoNotLock" false))

(event `Key|LeftMouseButton`
  (params (Key :type "Key Structure"))
  ;[1 1 1] Mouse Buttons Must Lock Mouse Again Every Release
  (:`Released`
    (`self.LockMouseToViewPort`)
    (`self.SelectedPasenger`
      (:`then`
        (if (not (`self.Controlling`))
          (`self.Set Selected Passenger` null)))
      (:`else`
        (`self.TrySelectPassanger`)))))

(event `Key|RightMouseButton`
  (params (Key :type "Key Structure"))
  ;[1 1 1] Mouse Buttons Must Lock Mouse Again Every Release
  (:`Released`
    (`self.LockMouseToViewPort`)
    (`self.SelectedPasenger`
      (:`then`
        (if (== (`.HitActor` (`GameplayStatics.BreakHitResult` (`PlayerController.GetHitResultUnderCursorForObjects` (`GameplayStatics.GetPlayerController` 0) (`|MakeArray` "ObjectTypeQuery3" :!type "EObjectTypeQuery Enum") true))) (`self.SelectedPasenger`))
          (set `self.Controlling` false)
          (bind _blackboardcomponent (`AIController.UseBlackboard` (`AIBlueprintHelperLibrary.GetAIController` (`self.SelectedPasenger`)) "/Game/AI/HellBoard.HellBoard"))
          (`BlackboardComponent.SetValueAsBool` _blackboardcomponent "Controlled" false)
          (`self.Set Selected Passenger` null)))
      (:`else`
        (bind _succes (`self.TrySelectPassanger`))
        (if _succes
          (set `self.Controlling` true)
          (bind _blackboardcomponent_2 (`AIController.UseBlackboard` (`AIBlueprintHelperLibrary.GetAIController` (`self.SelectedPasenger`)) "/Game/AI/HellBoard.HellBoard"))
          (`BlackboardComponent.SetValueAsBool` _blackboardcomponent_2 "Controlled" true))))))

(event `Key|Zero`
  (params (Key :type "Key Structure"))
  (:`Pressed`
    (`self.InitPlacement` "/Game/Blueprints/GridActor_Child.GridActor_Child_C")))

(event `Key|One`
  (params (Key :type "Key Structure"))
  (:`Pressed`
    (`self.InitPlacement` "/Game/Blueprints/BP_Bed.BP_Bed_C")))

(event `Key|Two`
  (params (Key :type "Key Structure"))
  (:`Pressed`
    (`self.InitPlacement` "/Game/Blueprints/BP_WorkStation.BP_WorkStation_C")))

(event `Key|Three`
  (params (Key :type "Key Structure"))
  (:`Pressed`
    (`self.InitPlacement` "/Game/Blueprints/BP_FoodStation.BP_FoodStation_C")))

(event `Key|LeftMouseButton`
  (params (Key :type "Key Structure"))
  (bind _spawnobject (`self.SpawnObject`))
  (:`Pressed`
    (`/Engine/EditorBlueprintResources/StandardMacros.IsValid` _spawnobject
      (:`Is Valid`
        (if (not (or (not (`/Game/Blueprints/BP_GridActor.CanBuild` _spawnobject)) (`/Game/Blueprints/BP_GridActor.BadTerrain` _spawnobject)))
          (`/Game/Blueprints/BP_GridActor.RemoveGrid` _spawnobject)
          (`KismetSystemLibrary.K2_ClearTimer` null "FollowMouse")
          (set `self.SpawnObject` null))))))

(event `Key|R`
  (params (Key :type "Key Structure"))
  (bind _spawnobject (`self.SpawnObject`))
  (:`Pressed`
    (`/Engine/EditorBlueprintResources/StandardMacros.IsValid` _spawnobject
      (:`Is Valid`
        (`SceneComponent.K2_AddWorldRotation` (`/Game/Blueprints/BP_GridActor.Scene` _spawnobject) (struct :`Yaw` 90.0) false false)))))

(fn `FollowMouse`
  (bind _spawnobject (`self.SpawnObject`))
  (bind (_bblockinghit _binitialoverlap _time _distance _location _impactpoint _normal _impactnormal _physmat _hitactor) (`GameplayStatics.BreakHitResult` (`PlayerController.GetHitResultUnderCursorByChannel` (`GameplayStatics.GetPlayerController` 0) "TraceTypeQuery1" true)))
  (cast `/Game/Blueprints/BP_Floor` _hitactor
    (:`then`
      (set `/Game/Blueprints/BP_GridActor.CanBuild` true _spawnobject)
      (`self.SetActorHiddenInGame` _spawnobject false))
    (:`CastFailed`
      (set `/Game/Blueprints/BP_GridActor.CanBuild` false _spawnobject)
      (`self.SetActorHiddenInGame` _spawnobject true)))
  (bind _outsnaptolocation (`self.SnapToGrid` _location 100))
  (`self.K2_SetActorLocation` (`self.SpawnObject`) _outsnaptolocation false false))

(fn `InitPlacement`
  (params (GridActorClass :type "/Game/Blueprints/BP_GridActor Class Reference"))
  (bind _spawnobject (`self.SpawnObject`))
  (`/Engine/EditorBlueprintResources/StandardMacros.IsValid` _spawnobject
    (:`Is Valid`
      (`self.K2_DestroyActor` _spawnobject)
      (set `self.SpawnObject` null))
    (:`Is Not Valid`
      _))
  (bind _outsnaptolocation (`self.SnapToGrid` (`self.K2_GetActorLocation`)))
  (bind _returnvalue (`|SpawnActorFromClass` (`local.GridActorClass`) (`KismetMathLibrary.Conv_VectorToTransform` _outsnaptolocation) "AdjustIfPossibleButDontSpawnIfColliding" "OverrideRootScale" null null))
  (set `self.SpawnObject` _returnvalue)
  (`KismetSystemLibrary.K2_SetTimer` null "FollowMouse" 0.01 true))

(fn `MovePassenger`
  (params (Hit :type "HitResult Structure"))
  (bind (_bblockinghit _binitialoverlap _time _distance _location) (`GameplayStatics.BreakHitResult` Hit))
  (`self.SelectedPasenger`
    (:`then`
      (if (>= (`KismetMathLibrary.VSize` (- (`self.K2_GetActorLocation` (`self.SelectedPasenger`)) _location)) 120.0)
        (`AIBlueprintHelperLibrary.SimpleMoveToLocation` (`AIBlueprintHelperLibrary.GetAIController` (`self.SelectedPasenger`)) _location)))
    (:`else`)))

(fn `Set Selected Passenger`
  (params (Pass :type "/Game/Blueprints/Passenger Object Reference"))
  (bind _pass (`local.Pass`))
  (`/Engine/EditorBlueprintResources/StandardMacros.IsValid` Pass
    (:`Is Valid`
      (if (not (`/Game/Blueprints/Passenger.IsDead` (`local.Pass`)))
        (`PrimitiveComponent.SetRenderCustomDepth` (`Character.Mesh` _pass) true)
        (set `self.SelectedPasenger` _pass)))
    (:`Is Not Valid`
      (bind _selectedpasenger (`self.SelectedPasenger`)
        (:`then`
          (`PrimitiveComponent.SetRenderCustomDepth` (`Character.Mesh` _selectedpasenger) false))
        (:`else`
          _))
      (set `self.SelectedPasenger` null))))

(fn `SnapToGrid`
  (params (InActorLocation :type "Vector Structure") (InGridSize :type Integer))
  (returns (OutSnapToLocation :type "Vector Structure"))
  (bind _x (.x InActorLocation))
  (bind _y (.y InActorLocation))
  (return (`KismetMathLibrary.MakeVector` (`KismetMathLibrary.Conv_IntToDouble` (* (/ (`KismetMathLibrary.FFloor` (+ _x (- _x (`KismetMathLibrary.Conv_IntToDouble` (* (/ (`KismetMathLibrary.FFloor` _x) InGridSize) InGridSize))))) InGridSize) InGridSize)) (`KismetMathLibrary.Conv_IntToDouble` (* (/ (`KismetMathLibrary.FFloor` (+ _y (- _y (`KismetMathLibrary.Conv_IntToDouble` (* (/ (`KismetMathLibrary.FFloor` _y) InGridSize) InGridSize))))) InGridSize) InGridSize)) (.z InActorLocation))))

(fn `TrySelectPassanger`
  (returns (Succes :type Boolean))
  (bind (_hitresult _returnvalue) (`PlayerController.GetHitResultUnderCursorForObjects` (`GameplayStatics.GetPlayerController` 0) (`|MakeArray` "ObjectTypeQuery3" :!type "EObjectTypeQuery Enum") true))
  (if _returnvalue
    (bind _aspassenger (cast `/Game/Blueprints/Passenger` (`.HitActor` (`GameplayStatics.BreakHitResult` _hitresult)))
      (:`then`
        (if (not (`/Game/Blueprints/Passenger.IsDead` _aspassenger))
          (`self.Set Selected Passenger` _aspassenger)
          (return true)))
      (:`CastFailed`
        (`self.Set Selected Passenger` null :!label _label)
        (return false)))
    (else
      (goto _label))))

(fn `UserConstructionScript`)