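; GridActor is a building placement footprint that shows whether the spot it occupies is clear.
; While unbuilt, GridBoundaries records overlapping actors in OverlappedWith, setting BadTerrain and the bad-terrain material until the last one leaves.
; RemoveGrid marks it Built, freezing that feedback and hiding the boundary mesh, which the author notes still lets other grids detect it.
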(event `RemoveGrid`
  (set `self.Built` true)
  ;[1 1 1] Change grid mat or set to invisible but grid will still detect other grid
  (`SceneComponent.SetVisibility` (`self.GridBoundaries`) false false))

(event `self.GridBoundaries.OnComponentBeginOverlap`
  (params (OverlappedComponent :type "PrimitiveComponent Object Reference") (OtherActor :type "Actor Object Reference") (OtherComp :type "PrimitiveComponent Object Reference") (OtherBodyIndex :type Integer) (bFromSweep :type Boolean) (SweepResult :type "HitResult Structure (by ref)"))
  ;[1 1 1] Making sure grid does not change color after building is placed
  (if (not (`self.Built`))
    ;[1 1 1] Fix for overlapping issue
    (`KismetArrayLibrary.Array_Add` (`self.OverlappedWith`) OtherActor)
    (set `self.BadTerrain` true)
    (`PrimitiveComponent.SetMaterial` (`self.GridBoundaries`) 0 "/Game/Materials/GridActorBadTerrainMat.GridActorBadTerrainMat")))

(event `self.GridBoundaries.OnComponentEndOverlap`
  (params (OverlappedComponent :type "PrimitiveComponent Object Reference") (OtherActor :type "Actor Object Reference") (OtherComp :type "PrimitiveComponent Object Reference") (OtherBodyIndex :type Integer))
  ;[1 1 1] Making sure grid does not change color after building is placed
  (if (not (`self.Built`))
    ;[1 1 1] Fix for overlapping issue
    (`KismetArrayLibrary.Array_RemoveItem` (`self.OverlappedWith`) OtherActor)
    (if (== (`KismetArrayLibrary.Array_Length` (`self.OverlappedWith`)) 0)
      (set `self.BadTerrain` false)
      (`PrimitiveComponent.SetMaterial` (`self.GridBoundaries`) 0 "/Game/Materials/GridActorGoodTerainMat.GridActorGoodTerainMat"))))

(fn `UserConstructionScript`)