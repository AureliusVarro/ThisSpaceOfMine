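; Game mode Blueprint that tracks the Food and Energy resources and shows them on the HUD.
; AddFood and AddEnergy apply a delta, clamp between zero and the maximum, and push the new value to the HUD's ResourcesDisplay when the HUD reference is valid.
; InitHUD stores the HUD reference and calls both with zero to refresh the display.
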(fn `AddEnergy`
  (params (DeltaEnergy :type Integer))
  (bind _output_get (set `self.Energy` (`KismetMathLibrary.Clamp` (+ (`self.Energy`) DeltaEnergy) 0 (`self.MaxEnergy`))))
  (bind _hud_ref (`self.HUD_Ref`)
    (:`then`
      (`/Game/Blueprints/UI/ResourcesDisplay.SetEnergy` (`/Game/Blueprints/UI/HUD.ResourcesDisplay` _hud_ref) _output_get))
    (:`else`)))

(fn `AddFood`
  (params (DeltaFood :type Integer))
  (bind _output_get (set `self.Food` (`KismetMathLibrary.Clamp` (+ (`self.Food`) DeltaFood) 0 (`self.MaxFood`))))
  (bind _hud_ref (`self.HUD_Ref`)
    (:`then`
      (`/Game/Blueprints/UI/ResourcesDisplay.SetFood` (`/Game/Blueprints/UI/HUD.ResourcesDisplay` _hud_ref) _output_get))
    (:`else`)))

(fn `InitHUD`
  (params (HUD_Ref :type "/Game/Blueprints/UI/HUD Object Reference"))
  (set `self.HUD_Ref` HUD_Ref)
  (`self.AddEnergy` 0)
  (`self.AddFood` 0))

(fn `UserConstructionScript`)